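; Player character Blueprint that enables normal input, drives a stand-in third-person camera and plays movement foley.
; UpdateCamera picks a far, close or aim style from the traversal component's strafe and aim state, snapping on possession and interpolating spring arm and FOV each tick.
; Jump and land events play gameplay-tagged sounds from a foley bank, with volume scaled by speed, for steadier timing than Motion Matching animation notifies.
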(event `self.ReceiveBeginPlay`
  (bind _assnplayer_controller (cast `SNPlayerController` (`GameplayStatics.GetPlayerController` 0)))
  (`SNPlayerController.EnabledInputType` _assnplayer_controller "Normal" true))

(event `self.ReceivePossessed`
  (params (NewController :type "Controller Object Reference"))
  ;[1 1 1] Event Possesed
  (`self.UpdateCamera` false))

(event `self.ReceiveTick`
  (params (DeltaSeconds :type "Float (single-precision)"))
  ;[1 1 1] Event Tick
  (`self.UpdateCamera` true))

(event `self.OnJumped`
  ;[1 1 1] Event On Jumped - Play a sound whenever the character jumps. This could be done with audio events on the jump animations, but this way gives us more consistent timing, since Motion Matching can pick different entry frames of the jump animations.
  (`self.PlayAudioEvent` (struct :`TagName` "Foley.Event.Jump") (`KismetMathLibrary.MapRangeClamped` (`KismetMathLibrary.VSizeXY` (`MovementComponent.Velocity` (`self.CharacterMovement`))) 0.0 500.0 0.5 1.0)))

(event `self.OnLanded`
  (params (Hit :type "HitResult Structure (by ref)"))
  (bind (_returnvalue_x _returnvalue_y _returnvalue_z) (`KismetMathLibrary.BreakVector` (`SNTraversalComponent.GetLandSpeed` (`self.GetTraversalComponent`))))
  ;[1 1 1] Event On Land - Play a sound whenever the character lands similar to Event On Jumped. This logic also caches the land velocity and enables a Just Landed flag, which is used in a Chooser Table asset to select landing databases. We want this flag to be true for more than one frame, so that if movement conditions change upon landing, such as starting or stopping right after impact, landing databases will still be valid.
  (`self.PlayAudioEvent` (struct :`TagName` "Foley.Event.Land") (`KismetMathLibrary.MapRangeClamped` _returnvalue_z -500.0 -900.0 0.5 1.5)))

(fn `CanPlayFootstepSounds`
  (returns (ReturnValue :type Boolean))
  (return (or (`NavMovementComponent.IsMovingOnGround` (`self.CharacterMovement`)) (`SNTraversalComponent.IsDoingTraversalAction` (`self.GetTraversalComponent`)))))

(fn `GetFoleyAudioBank`
  (returns (FoleyAudioBank :type "/SNAnimation/NoRelease/Audio/Foley/DABP_FoleyAudioBank Object Reference"))
  (return "/SNAnimation/NoRelease/Audio/Foley/DefaultFoleyEventAudioBank.DefaultFoleyEventAudioBank"))

(fn `PlayAudioEvent`
  (params (Value :type "GameplayTag Structure") (VolumeMultiplier :type "Float (single-precision)" :default 1.0) (PitchMultiplier :type "Float (single-precision)" :default 1.0))
  (bind _foleyaudiobank (`self.GetFoleyAudioBank`))
  (`GameplayStatics.PlaySoundAtLocation` (`/SNAnimation/NoRelease/Audio/Foley/DABP_FoleyAudioBank.GetSoundFromFoleyEvent` _foleyaudiobank Value) (`SceneComponent.K2_GetComponentLocation` (`self.Mesh`)) (struct) VolumeMultiplier PitchMultiplier 0.0 null null null null))

(fn `UpdateCamera`
  (params (Interpolate :type Boolean))
  (locals (TargetCameraParams :type "/SNAnimation/Blueprint/Data/S_SimpleCameraParams Structure" :default (struct :`SpringArmLength` 300.0 :`SocketOffset` (0.0 0.0 0.0) :`TranslationLagSpeed` 10.0 :`FieldOfView` 90.0 :`TransitionSpeed` 10.0)))
  (bind _cameradistancemultiplier (`self.CameraDistanceMultiplier`))
  (bind (_targetcameraparams_springarmlength _targetcameraparams_socketoffset _targetcameraparams_translationlagspeed _targetcameraparams_fieldofview _targetcameraparams_transitionspeed) (break `/SNAnimation/Blueprint/Data/S_SimpleCameraParams` (`local.TargetCameraParams`)))
  (bind (_targetcameraparams_springarmlength_2 _targetcameraparams_socketoffset_2 _targetcameraparams_translationlagspeed_2 _targetcameraparams_fieldofview_2 _targetcameraparams_transitionspeed_2) (break `/SNAnimation/Blueprint/Data/S_SimpleCameraParams` (`local.TargetCameraParams`)))
  (bind (_targetcameraparams_springarmlength_3 _targetcameraparams_socketoffset_3 _targetcameraparams_translationlagspeed_3 _targetcameraparams_fieldofview_3 _targetcameraparams_transitionspeed_3) (break `/SNAnimation/Blueprint/Data/S_SimpleCameraParams` (`local.TargetCameraParams`)))
  (bind _interpolate (`local.Interpolate`))
  (bind (_targetcameraparams_springarmlength_4 _targetcameraparams_socketoffset_4 _targetcameraparams_translationlagspeed_4 _targetcameraparams_fieldofview_4 _targetcameraparams_transitionspeed_4) (break `/SNAnimation/Blueprint/Data/S_SimpleCameraParams` (`local.TargetCameraParams`)))
  (bind (_springarmlength _socketoffset _translationlagspeed _fieldofview _transitionspeed) (break `/SNAnimation/Blueprint/Data/S_SimpleCameraParams` (select `bool` (`SNTraversalComponent.GetWantsToStrafe` (`self.GetTraversalComponent`)) :`false` (`self.CamStyle_Far`) :`true` (select `bool` (`SNTraversalComponent.GetWantsToAim` (`self.GetTraversalComponent`)) :`false` (`self.CamStyle_Close`) :`true` (`self.CamStyle_Aim`)))))
  ;[1 1 1] This function simply interpolates the Spring Arm values based on current character states, and is meant to serve as a stand-in for a true gameplay camera system.
  (set `local.TargetCameraParams` (make `/SNAnimation/Blueprint/Data/S_SimpleCameraParams` (* _springarmlength _cameradistancemultiplier) (* _socketoffset _cameradistancemultiplier) (`KismetMathLibrary.SelectFloat` _translationlagspeed -1.0 _interpolate) _fieldofview (`KismetMathLibrary.SelectFloat` _transitionspeed -1.0 _interpolate)))
  (bind _output_get (set `CameraComponent.FieldOfView` (`KismetMathLibrary.FInterpTo` (stale _output_get) _targetcameraparams_fieldofview (`GameplayStatics.GetWorldDeltaSeconds`) _targetcameraparams_transitionspeed) (`self.Camera`)))
  (bind _output_get_2 (set `SpringArmComponent.TargetArmLength` (`KismetMathLibrary.FInterpTo` (stale _output_get_2) _targetcameraparams_springarmlength_2 (`GameplayStatics.GetWorldDeltaSeconds`) _targetcameraparams_transitionspeed_2) (`self.SpringArm`)))
  (bind _output_get_3 (set `SpringArmComponent.CameraLagSpeed` (`KismetMathLibrary.FInterpTo` (stale _output_get_3) _targetcameraparams_translationlagspeed_3 (`GameplayStatics.GetWorldDeltaSeconds`) _targetcameraparams_transitionspeed_3) (`self.SpringArm`)))
  (bind _output_get_4 (set `SpringArmComponent.SocketOffset` (`KismetMathLibrary.VInterpTo` (stale _output_get_4) _targetcameraparams_socketoffset_4 (`GameplayStatics.GetWorldDeltaSeconds`) _targetcameraparams_transitionspeed_4) (`self.SpringArm`))))

(fn `UserConstructionScript`)